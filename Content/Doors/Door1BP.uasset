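; Door controller Blueprint that slides four level doors upward as their open flags are set in the game state.
; Every Tick it reads the flags from MyGameStateBP and raises actors in MyGameModeBP's DoorList by a fixed per-frame step up to a height limit, making speed frame-rate dependent.
; Checks are nested, so each door requires all preceding flags.
; A DoOnce per door plays the sliding sound once.
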(event EventBeginPlay)

(event EventTick
  (params (DeltaSeconds :type Float%20%28single-precision%29))
  (bind _asmy_game_state_bp (Utilities|Casting|CastToMyGameStateBP (Game|GetGameState)))
  (bind _output_get (Variables|Default|SetMyGameState _asmy_game_state_bp))
  (bind _asmy_game_mode_bp (Utilities|Casting|CastToMyGameModeBP (Game|GetGameMode)))
  (bind _output_get_2 (Variables|Default|SetMyGameMode _asmy_game_mode_bp))
  ;[1 1 1] open door 1
  (if (Variables|/Script/GameProject.MyGameState|GetopenDoor1 _output_get)
    (if (<= (.z (Transformation|GetActorLocation (Utilities|Array|Get(acopy) (Variables|/Game/Blueprints/MyGameModeBP.MyGameModeBP_C|GetDoorList _output_get_2)))) 2e+02)
      (Transformation|SetActorLocation (Utilities|Array|Get(acopy) (Variables|/Game/Blueprints/MyGameModeBP.MyGameModeBP_C|GetDoorList _output_get_2)) (Math|Vector|MakeVector (.x (Transformation|GetActorLocation (Utilities|Array|Get(acopy) (Variables|/Game/Blueprints/MyGameModeBP.MyGameModeBP_C|GetDoorList _output_get_2)))) (.y (Transformation|GetActorLocation (Utilities|Array|Get(acopy) (Variables|/Game/Blueprints/MyGameModeBP.MyGameModeBP_C|GetDoorList _output_get_2)))) (+ (.z (Transformation|GetActorLocation (Utilities|Array|Get(acopy) (Variables|/Game/Blueprints/MyGameModeBP.MyGameModeBP_C|GetDoorList _output_get_2)))) 1.05)) false false)
      (Utilities|FlowControl|DoOnce false
        (:Completed
          (Audio|PlaySoundatLocation "/Game/Sounds/SlidingDoor.SlidingDoor" (Transformation|GetActorLocation (Utilities|Array|Get(acopy) (Variables|/Game/Blueprints/MyGameModeBP.MyGameModeBP_C|GetDoorList _output_get_2)))))))
    ;[1 1 1] open door 2
    (if (Variables|/Script/GameProject.MyGameState|GetopenDoor2 (Variables|Default|GetMyGameState))
      (if (<= (.z (Transformation|GetActorLocation (Utilities|Array|Get(acopy) (Variables|/Game/Blueprints/MyGameModeBP.MyGameModeBP_C|GetDoorList (Variables|Default|GetMyGameMode)) 1))) 2e+02)
        (Transformation|SetActorLocation (Utilities|Array|Get(acopy) (Variables|/Game/Blueprints/MyGameModeBP.MyGameModeBP_C|GetDoorList (Variables|Default|GetMyGameMode)) 1) (Math|Vector|MakeVector (.x (Transformation|GetActorLocation (Utilities|Array|Get(acopy) (Variables|/Game/Blueprints/MyGameModeBP.MyGameModeBP_C|GetDoorList (Variables|Default|GetMyGameMode)) 1))) (.y (Transformation|GetActorLocation (Utilities|Array|Get(acopy) (Variables|/Game/Blueprints/MyGameModeBP.MyGameModeBP_C|GetDoorList (Variables|Default|GetMyGameMode)) 1))) (+ (.z (Transformation|GetActorLocation (Utilities|Array|Get(acopy) (Variables|/Game/Blueprints/MyGameModeBP.MyGameModeBP_C|GetDoorList (Variables|Default|GetMyGameMode)) 1))) 1.05)) false false)
        (Utilities|FlowControl|DoOnce false
          (:Completed
            (Audio|PlaySoundatLocation "/Game/Sounds/SlidingDoor.SlidingDoor" (Transformation|GetActorLocation (Utilities|Array|Get(acopy) (Variables|/Game/Blueprints/MyGameModeBP.MyGameModeBP_C|GetDoorList (Variables|Default|GetMyGameMode)) 1))))))
      ;[1 1 1] open door 3
      (if (Variables|/Script/GameProject.MyGameState|GetopenDoor3 (Variables|Default|GetMyGameState))
        (if (<= (.z (Transformation|GetActorLocation (Utilities|Array|Get(acopy) (Variables|/Game/Blueprints/MyGameModeBP.MyGameModeBP_C|GetDoorList (Variables|Default|GetMyGameMode)) 2))) 2e+02)
          (Transformation|SetActorLocation (Utilities|Array|Get(acopy) (Variables|/Game/Blueprints/MyGameModeBP.MyGameModeBP_C|GetDoorList (Variables|Default|GetMyGameMode)) 2) (Math|Vector|MakeVector (.x (Transformation|GetActorLocation (Utilities|Array|Get(acopy) (Variables|/Game/Blueprints/MyGameModeBP.MyGameModeBP_C|GetDoorList (Variables|Default|GetMyGameMode)) 2))) (.y (Transformation|GetActorLocation (Utilities|Array|Get(acopy) (Variables|/Game/Blueprints/MyGameModeBP.MyGameModeBP_C|GetDoorList (Variables|Default|GetMyGameMode)) 2))) (+ (.z (Transformation|GetActorLocation (Utilities|Array|Get(acopy) (Variables|/Game/Blueprints/MyGameModeBP.MyGameModeBP_C|GetDoorList (Variables|Default|GetMyGameMode)) 2))) 1.05)) false false)
          (Utilities|FlowControl|DoOnce false
            (:Completed
              (Audio|PlaySoundatLocation "/Game/Sounds/SlidingDoor.SlidingDoor" (Transformation|GetActorLocation (Utilities|Array|Get(acopy) (Variables|/Game/Blueprints/MyGameModeBP.MyGameModeBP_C|GetDoorList (Variables|Default|GetMyGameMode)) 2))))))
        ;[1 1 1] open door 4
        (if (Variables|/Script/GameProject.MyGameState|GetopenDoor4 (Variables|Default|GetMyGameState))
          (if (<= (.z (Transformation|GetActorLocation (Utilities|Array|Get(acopy) (Variables|/Game/Blueprints/MyGameModeBP.MyGameModeBP_C|GetDoorList (Variables|Default|GetMyGameMode)) 3))) 2e+02)
            (Transformation|SetActorLocation (Utilities|Array|Get(acopy) (Variables|/Game/Blueprints/MyGameModeBP.MyGameModeBP_C|GetDoorList (Variables|Default|GetMyGameMode)) 3) (Math|Vector|MakeVector (.x (Transformation|GetActorLocation (Utilities|Array|Get(acopy) (Variables|/Game/Blueprints/MyGameModeBP.MyGameModeBP_C|GetDoorList (Variables|Default|GetMyGameMode)) 3))) (.y (Transformation|GetActorLocation (Utilities|Array|Get(acopy) (Variables|/Game/Blueprints/MyGameModeBP.MyGameModeBP_C|GetDoorList (Variables|Default|GetMyGameMode)) 3))) (+ (.z (Transformation|GetActorLocation (Utilities|Array|Get(acopy) (Variables|/Game/Blueprints/MyGameModeBP.MyGameModeBP_C|GetDoorList (Variables|Default|GetMyGameMode)) 3))) 1.05)) false false)
            (Utilities|FlowControl|DoOnce false
              (:Completed
                (Audio|PlaySoundatLocation "/Game/Sounds/SlidingDoor.SlidingDoor" (Transformation|GetActorLocation (Utilities|Array|Get(acopy) (Variables|/Game/Blueprints/MyGameModeBP.MyGameModeBP_C|GetDoorList (Variables|Default|GetMyGameMode)) 3)))))))))))

(fn ConstructionScript)