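; Enemy character with a health bar, pawn sensing and a collectable drop on death.
; Tick updates the widget's health bar and turns it toward the player.
; Only player damage reduces Health; at zero the enemy is destroyed, spawning a collectable sphere if IsInRoom was set by any capsule overlap.
; Damage or sight sets ThreatNoted, with a retriggerable delay clearing it shortly after the last sighting.
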(event OnSeePawn(PawnSensing)
  (params (Pawn :type Pawn%20Object%20Reference))
  ;[1 1 1] Enemy Sees Player
  (Variables|Default|SetInstigatedObject (Pawn|GetController Pawn))
  (Utilities|FlowControl|Sequence
    (:then_0
      (Variables|Default|SetThreatNoted true))
    (:then_1
      (Utilities|FlowControl|RetriggerableDelay 0.6)
      (Variables|Default|SetThreatNoted false))))

(event OnComponentBeginOverlap(CapsuleComponent)
  (params (OverlappedComponent :type Primitive%20Component%20Object%20Reference) (OtherActor :type Actor%20Object%20Reference) (OtherComp :type Primitive%20Component%20Object%20Reference) (OtherBodyIndex :type Integer) (bFromSweep :type Boolean) (SweepResult :type Hit%20Result%20Structure%20%28by%20ref%29))
  (Variables|Default|SetIsInRoom true))

(event Game|Damage|EventAnyDamage
  (params (Damage :type Float%20%28single-precision%29) (DamageType :type Damage%20Type%20Object%20Reference) (InstigatedBy :type Controller%20Object%20Reference) (DamageCauser :type Actor%20Object%20Reference))
  (bind _returnvalue (Transformation|GetActorTransform))
  (bind _widgetscenecomp (Variables|Default|GetWidgetSceneComp))
  (bind (_x _y _z) (Math|Vector|BreakVector (.location _returnvalue)))
  (bind _output_get (Variables|Default|SetInstigatedObject InstigatedBy))
  (if (== _output_get (Game|GetPlayerController 0))
    ;[1 1 1] Enemy Takes Damage From Player
    (Variables|Default|SetThreatNoted true)
    (bind _output_get_2 (Variables|Default|SetHealth (- (Variables|Default|GetHealth) Damage)))
    (bind _asenemy_health (Utilities|Casting|CastToEnemyHealth (UserInterface|GetUserWidgetObject (Variables|Default|GetWidget))))
    (Progress|SetPercent (Variables|/Game/Hud/EnemyHealth.EnemyHealth_C|GetProgressBar_175 _asenemy_health) (/ _output_get_2 1e+02))
    (Transformation|SetWorldRotation _widgetscenecomp (Math|Rotator|FindLookatRotation (Transformation|GetWorldLocation _widgetscenecomp) (Transformation|GetActorLocation (Game|GetPlayerCharacter 0))) false false)
    (if (<= _output_get_2 0.0)
      (if (Variables|Default|GetIsInRoom)
        (Game|SpawnActorfromClass "/Game/Blueprints/CollectableSphereBP.CollectableSphereBP_C" (Math|Transform|MakeTransform (Math|Vector|MakeVector _x _y (+ (- _z (.z (Transformation|GetActorLocation))) 2e+01)) (.rotation _returnvalue) (.scale _returnvalue)) "Undefined" 0 0)
        (Actor|DestroyActor)
        (else
          (Actor|DestroyActor))))))

(event EventTick
  (params (DeltaSeconds :type Float%20%28single-precision%29))
  (bind _widgetscenecomp (Variables|Default|GetWidgetSceneComp))
  ;[1 1 1] Initialize Health Widget
  (bind _asenemy_health (Utilities|Casting|CastToEnemyHealth (UserInterface|GetUserWidgetObject (Variables|Default|GetWidget))))
  (Progress|SetPercent (Variables|/Game/Hud/EnemyHealth.EnemyHealth_C|GetProgressBar_175 _asenemy_health) (/ (Variables|Default|GetHealth) 1e+02))
  (Transformation|SetWorldRotation _widgetscenecomp (Math|Rotator|FindLookatRotation (Transformation|GetWorldLocation _widgetscenecomp) (Transformation|GetActorLocation (Game|GetPlayerCharacter 0))) false false))

(fn ConstructionScript)