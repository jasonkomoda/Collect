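; Game mode Blueprint that populates the level with enemies, doors and a first collectable sphere on BeginPlay.
; Each enemy spawns at a listed point, gets its default AI controller, runs the EnemyBT behavior tree and joins EnemyCharacterList.
; Doors spawn from two location arrays, the second set rotated 90 degrees, and collect in DoorList.
; The sphere spawns last at a hard-coded location.
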(event EventBeginPlay
  (bind _doorlist (Variables|Default|GetDoorList))
  ;[1 1 1] spawn enemies
  (for _array_element (Variables|Default|GetEnemySpawnPoints)
    (bind _returnvalue (Game|SpawnActorfromClass "/Game/Enemy/EnemyCharacter_BP.EnemyCharacter_BP_C" (Math|Transform|MakeTransform _array_element "0,0.000000, 0") "AlwaysSpawn" 0 0))
    (Pawn|SpawnDefaultController _returnvalue)
    (bind _asenemy_ai_bp (Utilities|Casting|CastToEnemyAI_BP (Pawn|GetController _returnvalue)))
    (AI|RunBehaviorTree _asenemy_ai_bp "/Game/Enemy/EnemyBT.EnemyBT")
    (Utilities|Array|Add (Variables|Default|GetEnemyCharacterList) _returnvalue))
  ;[1 1 1] spawn doors
  (for _array_element_2 (Variables|Default|GetFirstTwoDoorSpawnPoints)
    (bind _returnvalue_2 (Game|SpawnActorfromClass "/Game/Doors/Door1BP.Door1BP_C" (Math|Transform|MakeTransform _array_element_2 "0, 0, 0" "1.000000,1,1") "Undefined" 0 0))
    (Utilities|Array|Add _doorlist _returnvalue_2))
  (for _array_element_3 (Variables|Default|GetSecondTwoDoorSpawnPoints)
    (bind _returnvalue_3 (Game|SpawnActorfromClass "/Game/Doors/Door1BP.Door1BP_C" (Math|Transform|MakeTransform _array_element_3 "0,90.000000, 0") "Undefined" 0 0))
    (Utilities|Array|Add _doorlist _returnvalue_3))
  ;[1 1 1] spawn first sphere
  (Game|SpawnActorfromClass "/Game/Blueprints/CollectableSphereBP.CollectableSphereBP_C" (Math|Transform|MakeTransform "6700.000000,286.000000,20.000000") "Undefined" 0 0))

(fn ConstructionScript)