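; Player character Blueprint with aim-down-sights shooting, swim forward input, damage handling and sphere-pickup feedback.
; Aiming tightens the camera, switches to control rotation and shows a crosshair, enabling automatic hitscan fire through a looping Gate and retriggerable delay.
; Damage lowers GameState health, pausing with a Game Over screen at zero.
; Tick polls a flag to play pickup sounds and show the go-outside prompt once enough spheres are collected.
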(event Custom|StopFire
  (bind _followcamera (Variables|Default|GetFollowCamera))
  (bind _returnvalue (Transformation|GetWorldLocation _followcamera))
  ;[1 1 1] Shoot Weapon
  (Utilities|FlowControl|Gate true) ; enters at Close
)

(event Custom|Fire
  (bind _followcamera (Variables|Default|GetFollowCamera))
  (bind _returnvalue (Transformation|GetWorldLocation _followcamera))
  ;[1 1 1] Shoot Weapon
  (Utilities|FlowControl|Sequence
    (:then_0
      (goto _label Open))
    (:then_1
      (Utilities|FlowControl|Gate true :!label _label
        (:Exit
          (Utilities|FlowControl|Sequence
            (:then_0
              (Utilities|FlowControl|RetriggerableDelay 0.1)
              (goto _label))
            (:then_1
              (bind (_outhit _returnvalue_2) (Collision|LineTraceByChannel _returnvalue (+ _returnvalue (* (Math|Vector|GetForwardVector (Transformation|GetWorldRotation _followcamera)) 2.5e+04)) "TraceTypeQuery1" false 0 "None"))
              (if _returnvalue_2
                (Audio|SpawnSoundatLocation "/Game/Sounds/GunSound.GunSound" (Transformation|GetActorLocation))
                (Effects|SpawnEmitteratLocation "/Game/StarterContent/Particles/P_Explosion.P_Explosion" (.Location (Collision|BreakHitResult _outhit)))
                (Game|Damage|ApplyDamage (.HitActor (Collision|BreakHitResult _outhit)) 5.0 (Pawn|GetController self) 0)))))))))

(event EventBeginPlay
  ;[1 1 1] Create Crosshair Widget
  (bind _asmy_hud (Utilities|Casting|CastToMyHud (HUD|GetHUD (Game|GetPlayerController 0))))
  (Variables|Default|SetMyHud _asmy_hud)
  (bind _asmy_game_state_bp (Utilities|Casting|CastToMyGameStateBP (Game|GetGameState)))
  (Variables|Default|SetMyGameState _asmy_game_state_bp))

(event Game|Damage|EventAnyDamage
  (params (Damage :type Float%20%28single-precision%29) (DamageType :type Damage%20Type%20Object%20Reference) (InstigatedBy :type Controller%20Object%20Reference) (DamageCauser :type Actor%20Object%20Reference))
  (bind _mygamestate (Variables|Default|GetMyGameState))
  ;[1 1 1] Player Takes Damage
  (Audio|PlaySoundatLocation "/Game/Sounds/PlayerGetsHit.PlayerGetsHit" (Transformation|GetActorLocation))
  (bind _output_get (Variables|/Script/GameProject.MyGameState|SetplayerHealth _mygamestate (- (Variables|/Script/GameProject.MyGameState|GetplayerHealth _mygamestate) Damage)))
  (if (<= _output_get 0.0)
    (Game|SetGamePaused true)
    (UserInterface|Viewport|AddtoViewport (Variables|/Game/Hud/MyHud.MyHud_C|GetGameOver (Variables|Default|GetMyHud)) 0)
    (bind _asmy_player_controller (Utilities|Casting|CastToMyPlayerController (Game|GetPlayerController 0)))
    (Variables|/Script/Engine.PlayerController|SetbShowMouseCursor _asmy_player_controller true)
    (Variables|/Script/Engine.PlayerController|SetbEnableClickEvents _asmy_player_controller true)
    (Variables|/Script/Engine.PlayerController|SetbEnableMouseOverEvents _asmy_player_controller true)))

(event EventTick
  (params (DeltaSeconds :type Float%20%28single-precision%29))
  ;[1 1 1] play collect sphere sound
  (if (Variables|Default|GetplaySound)
    (Audio|PlaySoundatLocation "/Game/Sounds/spherePickup.spherePickup" (Transformation|GetActorLocation))
    (Variables|Default|SetplaySound false)
    ;[1 1 1] show goOutside hud
    (if (>= (Variables|/Script/GameProject.MyGameState|GetNumSpheresCollected (Variables|Default|GetMyGameState)) 11)
      (Utilities|FlowControl|DoOnce false
        (:Completed
          (UserInterface|Viewport|AddtoViewport (Variables|/Game/Hud/MyHud.MyHud_C|GetGoOutside (Variables|Default|GetMyHud)) 0))))))

(event Input|ActionEvents|InputActionAttack
  (params (Key :type Key%20Structure :default "AnyKey"))
  (bind _isads (Variables|Default|GetIsADS))
  ;[1 1 1] Shoot Weapon
  (:Pressed
    (if _isads
      (Variables|Default|SetCanFire true)
      (CallFunction|Fire)))
  (:Released
    (if _isads
      (Variables|Default|SetCanFire false)
      (CallFunction|StopFire))))

(event Input|ActionEvents|InputActionAimDownSights
  (params (Key :type Key%20Structure :default "AnyKey"))
  (bind _myhud (Variables|Default|GetMyHud))
  (bind _followcamera (Variables|Default|GetFollowCamera))
  (bind _charactermovement (Variables|Character|GetCharacterMovement))
  (bind _cameraboom (Variables|Default|GetCameraBoom))
  (bind _crosshairaim (Variables|/Game/Hud/MyHud.MyHud_C|GetCrosshairAim _myhud))
  ;[1 1 1] AimDownSight
  (:Pressed
    (UserInterface|Viewport|AddtoViewport _crosshairaim 0)
    (Variables|Default|SetIsADS true)
    (Variables|/Script/Engine.SpringArmComponent|SetTargetArmLength _cameraboom 6e+01)
    (Camera|SetFieldOfView _followcamera 75.0)
    (bind _output_get (Variables|/Script/Engine.CameraComponent|SetbUsePawnControlRotation _followcamera true))
    (Variables|Default|SetbUseControllerRotationYaw _output_get)
    (Variables|/Script/Engine.CharacterMovementComponent|SetbOrientRotationToMovement _charactermovement false))
  (:Released
    (CallFunction|StopFire)
    (Widget|RemovefromParent _crosshairaim)
    (Variables|Default|SetIsADS false)
    (Variables|/Script/Engine.SpringArmComponent|SetTargetArmLength _cameraboom 1e+02)
    (Camera|SetFieldOfView _followcamera 9e+01)
    (bind _output_get_2 (Variables|/Script/Engine.CameraComponent|SetbUsePawnControlRotation _followcamera false))
    (Variables|Default|SetbUseControllerRotationYaw _output_get_2)
    (Variables|/Script/Engine.CharacterMovementComponent|SetbOrientRotationToMovement _charactermovement true)))

(event Input|AxisEvents|InputAxisMoveForward
  (params (AxisValue :type Float%20%28single-precision%29))
  ;[1 1 1] swim mode
  (if (Variables|Default|GetisSwimming)
    (Pawn|Input|AddMovementInput (Math|Vector|GetForwardVector (Math|Rotator|MakeRotator 0.0 0.0 (.Yaw (Math|Rotator|BreakRotator (Pawn|GetControlRotation :!class /Script/Engine.Pawn))))) AxisValue false)))

(fn ConstructionScript)